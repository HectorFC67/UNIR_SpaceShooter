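; BP_SS_HUD is the HUD Blueprint that shows the player's lives and game progress on screen.
; On BeginPlay it creates BP_SS_Widget for the first player controller, adds it to the viewport, and caches the BP_SS_Actor player character and SS_GameMode.
; Every Tick it polls Progress from the game mode and Lifes from the character and pushes both into the widget's UpdateWidget.
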(event `self.ReceiveBeginPlay`
  (bind _returnvalue (`GameplayStatics.GetPlayerController` 0))
  (`/Engine/EditorBlueprintResources/StandardMacros.IsValid` _returnvalue
    (:`Is Valid`
      (bind _returnvalue_2 (`|GenericCreateObject` _returnvalue "/Game/HUD/BP_SS_Widget.BP_SS_Widget_C"))
      (bind _output_get (set `self.GameWidget` _returnvalue_2))
      (`UserWidget.AddToViewport` _output_get 0)
      (bind _asbp_ss_actor (cast `/Game/Player/BP_SS_Actor` (`GameplayStatics.GetPlayerCharacter` 0)))
      (set `self.m_PlayerCharacter` _asbp_ss_actor)
      (bind _asss_game_mode (cast `/Game/Map/SS_GameMode` (`GameplayStatics.GetGameMode`)))
      (set `self.As SS Game Mode` _asss_game_mode))))

(event `self.ReceiveTick`
  (params (DeltaSeconds :type "Float (single-precision)"))
  (`/Game/HUD/BP_SS_Widget.UpdateWidget` (`self.GameWidget`) (`/Game/Map/SS_GameMode.Progress` (`self.As SS Game Mode`)) (`/Game/Player/BP_SS_Actor.Lifes` (`self.m_PlayerCharacter`))))

(fn `UserConstructionScript`)