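; BP_EnemyH is an enemy Blueprint that sets a sideways movement direction and reverses it at actors tagged "Lateral".
; It starts along its right vector, then each overlap with such an actor toggles IsRight and flips MovementVector.
; Each flip away from the right also shortens DelayShoot.
; Tick is disabled and the graph only sets these variables, calling parent logic on BeginPlay and overlap.
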(event `self.ReceiveBeginPlay`
  (`parent.ReceiveBeginPlay`)
  (set `self.MovementVector` (`self.GetActorRightVector`))
  (set `self.IsRight` true))

(event `self.ReceiveActorBeginOverlap`
  (params (OtherActor :type "Actor Object Reference"))
  (`parent.ReceiveActorBeginOverlap` OtherActor)
  (if (`KismetArrayLibrary.Array_Contains` (`Actor.Tags` OtherActor) "Lateral")
    (if (`self.IsRight`)
      (set `self.IsRight` false)
      (set `self.MovementVector` (* (stale _output_get) -1.0))
      (set `self.DelayShoot` (- (`self.DelayShoot`) 0.1))
      (else
        (set `self.IsRight` true)
        (bind _output_get (set `self.MovementVector` (`self.GetActorRightVector`)))))))

(fn `UserConstructionScript`
  (`parent.UserConstructionScript`))