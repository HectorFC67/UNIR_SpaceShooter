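; Player-controlled pawn that moves and fires projectiles through Enhanced Input.
; On BeginPlay it adds the player mapping context to its controller's input subsystem.
; The movement action feeds movement input along the pawn's right and forward vectors.
; The fire action spawns BP_SS_Ammo at the FirePoint transform, with a CanFire flag and a timer enforcing a delay between shots.
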(event `self.ReceiveBeginPlay`
  (bind _asplayer_controller (cast `PlayerController` (`self.GetController`)))
  (bind _returnvalue (pcsubsystem `EnhancedInputLocalPlayerSubsystem` _asplayer_controller))
  (`/Engine/EditorBlueprintResources/StandardMacros.IsValid` _returnvalue
    (:`Is Valid`
      (`EnhancedInputSubsystemInterface.AddMappingContext` _returnvalue "/Game/Input/IMC_Player.IMC_Player" 0 (struct)))))

(event `EnhancedInput|/Game/Input/IA_PlayerFire`
  (params (ActionValue :type Boolean) (ElapsedSeconds :type "Float (double-precision)") (TriggeredSeconds :type "Float (double-precision)") (InputAction :type "InputAction Object Reference" :default "/Game/Input/IA_PlayerFire.IA_PlayerFire"))
  (:`Triggered`
    (if (`self.CanFire`)
      (`self.Fire`)
      (set `self.CanFire` false)
      (`KismetSystemLibrary.K2_SetTimerDelegate` (delegate `EnableFire`) (`self.FireDelay`)))))

(event `EnableFire`
  (set `self.CanFire` true))

(event `EnhancedInput|/Game/Input/IA_PlayerMovement`
  (params (ActionValue :type "Vector2D Structure") (ElapsedSeconds :type "Float (double-precision)") (TriggeredSeconds :type "Float (double-precision)") (InputAction :type "InputAction Object Reference" :default "/Game/Input/IA_PlayerMovement.IA_PlayerMovement"))
  (:`Triggered`
    (`self.AddMovementInput` (`self.GetActorRightVector`) ActionValue_X)
    (`self.AddMovementInput` (`self.GetActorForwardVector`) ActionValue_Y)))

(fn `Fire`
  (`|SpawnActorFromClass` "/Game/Player/BP_SS_Ammo.BP_SS_Ammo_C" (`SceneComponent.K2_GetComponentToWorld` (`self.FirePoint`)) "Undefined" "MultiplyWithRoot" null null))

(fn `UserConstructionScript`)